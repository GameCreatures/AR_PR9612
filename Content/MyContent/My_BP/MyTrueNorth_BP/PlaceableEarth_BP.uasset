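; A placeable Earth actor that lets the player zoom to Puerto Rico by touch and travel to the San Juan level.
; On BeginPlay a timeline animates the Ground's scale.
; The first touch on the Cube runs a second timeline that scales Earth and the Puerto Rico parent, then hides Earth and swaps Puerto Rico to a non-pulsing material.
; Touching the static mesh opens OnSanjuan.
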(event `self.ReceiveBeginPlay`
  (bind (_direction _scaleanim) (`Timeline|Timeline_0`)
    (:`Update`
      (`SceneComponent.SetRelativeScale3D` (`self.Ground`) (`KismetMathLibrary.Conv_DoubleToVector` _scaleanim)))))

(event `self.Cube.OnInputTouchBegin`
  (params (FingerIndex :type "ETouchIndex Enum" :default "Touch1") (TouchedComponent :type "PrimitiveComponent Object Reference"))
  (bind _earth (`self.Earth`))
  (if (not (`self.bHasBeenTouched`))
    (`KismetSystemLibrary.PrintString` "Puerto Rico touched")
    (bind (_direction _scaleanim _puertoricoscalegrow) (`Timeline|Timeline_1` :!via `PlayFromStart`)
      (:`Update`
        (`SceneComponent.SetRelativeScale3D` _earth (`KismetMathLibrary.Conv_DoubleToVector` _scaleanim))
        (`SceneComponent.SetRelativeScale3D` (`self.PR_Parent`) (`KismetMathLibrary.Conv_DoubleToVector` _puertoricoscalegrow))
        (set `self.bHasBeenTouched` true))
      (:`Finished`
        (`SceneComponent.SetVisibility` _earth false false)
        (`PrimitiveComponent.SetMaterial` (`self.PuertoRico`) 0 "/Game/MyContent/Art/Textures/PuertoRicoTextures/PuertoRico_DiffusseNOPulse_Mat.PuertoRico_DiffusseNOPulse_Mat")))))

(event `self.StaticMesh.OnInputTouchBegin`
  (params (FingerIndex :type "ETouchIndex Enum" :default "Touch1") (TouchedComponent :type "PrimitiveComponent Object Reference"))
  (`GameplayStatics.OpenLevel` "OnSanjuan"))

(fn `UserConstructionScript`)